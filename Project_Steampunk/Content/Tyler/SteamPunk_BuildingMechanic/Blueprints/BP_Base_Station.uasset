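; BP_Base_Station is an interactable station for a steampunk building mechanic, made of five base platform meshes.
; LookatTrace highlights all five platforms by swapping their first material slot to AliasReference, and LookatTraceEnd sets them to WorldGridMaterial.
; OnInteract is a placeholder that only prints a message saying the building process begins.
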(event `/Game/Tyler/SteamPunk_BuildingMechanic/Interfaces/BPI_Interactable.OnInteract`
  (`KismetSystemLibrary.PrintString` "Building Process Begins!"))

(event `/Game/Tyler/SteamPunk_BuildingMechanic/Interfaces/BPI_Interactable.LookAtTrace`
  (`PrimitiveComponent.SetMaterial` (`self.BasePlatform`) 0 "/DatasmithContent/Materials/AliasReference.AliasReference")
  (`PrimitiveComponent.SetMaterial` (`self.BasePlatform3`) 0 "/DatasmithContent/Materials/AliasReference.AliasReference")
  (`PrimitiveComponent.SetMaterial` (`self.BasePlatform4`) 0 "/DatasmithContent/Materials/AliasReference.AliasReference")
  (`PrimitiveComponent.SetMaterial` (`self.BasePlatform1`) 0 "/DatasmithContent/Materials/AliasReference.AliasReference")
  (`PrimitiveComponent.SetMaterial` (`self.BasePlatform2`) 0 "/DatasmithContent/Materials/AliasReference.AliasReference"))

(event `/Game/Tyler/SteamPunk_BuildingMechanic/Interfaces/BPI_Interactable.LookAtTraceEnd`
  (`PrimitiveComponent.SetMaterial` (`self.BasePlatform`) 0 "/Engine/EngineMaterials/WorldGridMaterial.WorldGridMaterial")
  (`PrimitiveComponent.SetMaterial` (`self.BasePlatform3`) 0 "/Engine/EngineMaterials/WorldGridMaterial.WorldGridMaterial")
  (`PrimitiveComponent.SetMaterial` (`self.BasePlatform4`) 0 "/Engine/EngineMaterials/WorldGridMaterial.WorldGridMaterial")
  (`PrimitiveComponent.SetMaterial` (`self.BasePlatform1`) 0 "/Engine/EngineMaterials/WorldGridMaterial.WorldGridMaterial")
  (`PrimitiveComponent.SetMaterial` (`self.BasePlatform2`) 0 "/Engine/EngineMaterials/WorldGridMaterial.WorldGridMaterial"))

(fn `UserConstructionScript`)