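; Base object for the building mechanic that the first-person character can pick up, rotate, drop and snap onto other objects' connection points.
; Pickup attaches the mesh to the right-hand socket, while placement attaches it to the character's hit component.
; Parent and child references track connections, and an object counts as detachable only without children.
; Rotation steps 45 degrees around a switchable X/Z axis, and four attachment-point markers toggle visibility.
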(event `/Game/Tyler/SteamPunk_BuildingMechanic/Interfaces/BPI_Interactable.SwitchRotationAxis`
  (`/Engine/EditorBlueprintResources/StandardMacros.FlipFlop`
    (:`A`
      (set `self.CurrentAxisEnum` "Z"))
    (:`B`
      (set `self.CurrentAxisEnum` "X"))))

(event `self.ReceiveBeginPlay`
  (bind _asbp_first_person_character (cast `/Game/FirstPerson/Blueprints/BP_FirstPersonCharacter` (`GameplayStatics.GetPlayerCharacter` 0)))
  (set `self.BP_FirstPersonRef` _asbp_first_person_character))

(event `/Game/Tyler/SteamPunk_BuildingMechanic/Interfaces/BPI_Interactable.RotateObject`
  (bind _basemesh (`self.BaseMesh`))
  (bind _basemesh_2 (`self.BaseMesh`))
  (bind (_relativerotation_roll _relativerotation_pitch _relativerotation_yaw) (`KismetMathLibrary.BreakRotator` (`SceneComponent.RelativeRotation` _basemesh)))
  (bind (_relativerotation_roll_2 _relativerotation_pitch_2 _relativerotation_yaw_2) (`KismetMathLibrary.BreakRotator` (`SceneComponent.RelativeRotation` _basemesh_2)))
  (if (`|EnumEquality` (`self.CurrentAxisEnum`) "X")
    (`SceneComponent.K2_SetRelativeRotation` _basemesh (`KismetMathLibrary.MakeRotator` (+ _relativerotation_roll 45.0) _relativerotation_pitch _relativerotation_yaw) false false)
    (elif (`|EnumEquality` (`self.CurrentAxisEnum`) "Z")
      (`SceneComponent.K2_SetWorldRotation` _basemesh_2 (`KismetMathLibrary.MakeRotator` _relativerotation_roll_2 _relativerotation_pitch_2 (+ _relativerotation_yaw_2 45.0)) false false))))

(event `/Game/Tyler/SteamPunk_BuildingMechanic/Interfaces/BPI_Interactable.PickupObject`
  (if (not (`/Game/FirstPerson/Blueprints/BP_FirstPersonCharacter.IsObjectInHand?` (`self.BP_FirstPersonRef`)))
    (`PrimitiveComponent.SetSimulatePhysics` (`self.BaseMesh`) false)
    (`PrimitiveComponent.SetCollisionEnabled` (`self.BaseMesh`) "QueryAndPhysics")
    (`KismetSystemLibrary.Delay` 0.1)
    (bind _returnvalue (`SceneComponent.K2_AttachToComponent` (`self.BaseMesh`) (`/Game/FirstPerson/Blueprints/BP_FirstPersonCharacter.RightHandSocket` (`self.BP_FirstPersonRef`)) "None" "SnapToTarget" "SnapToTarget" "KeepWorld" true))
    (set `/Game/FirstPerson/Blueprints/BP_FirstPersonCharacter.IsObjectInHand?` _returnvalue (`self.BP_FirstPersonRef`))
    (`self.RemoveChildRefrence` null)))

(event `/Game/Tyler/SteamPunk_BuildingMechanic/Interfaces/BPI_Interactable.AttachToConnectionPoint`
  (`PrimitiveComponent.SetSimulatePhysics` (`self.BaseMesh`) false)
  (`PrimitiveComponent.SetCollisionEnabled` (`self.BaseMesh`) "NoCollision")
  (`SceneComponent.K2_AttachToComponent` (`self.BaseMesh`) (`/Game/FirstPerson/Blueprints/BP_FirstPersonCharacter.Out Hit Hit Component` (`self.BP_FirstPersonRef`)) "None" "SnapToTarget" "KeepWorld" "KeepWorld" false)
  (bind _asbp_base_object (cast `/Game/Tyler/SteamPunk_BuildingMechanic/Blueprints/BP_Base_Object` (`ActorComponent.GetOwner` (`/Game/FirstPerson/Blueprints/BP_FirstPersonCharacter.Out Hit Hit Component` (`self.BP_FirstPersonRef`)))))
  (bind _output_get (set `self.ParentObject` _asbp_base_object))
  (`self.AddChildRefrence` _output_get self)
  (`PrimitiveComponent.SetCollisionEnabled` (`self.BaseMesh`) "QueryOnly"))

(event `/Game/Tyler/SteamPunk_BuildingMechanic/Interfaces/BPI_Interactable.HideAttachmentPoints`
  (for _array_element (`|MakeArray` (`self.Front`) (`self.Top`) (`self.Bottom`) (`self.Back`))
    (`SceneComponent.SetVisibility` (`SceneComponent.GetChildComponent` _array_element 0) false false)))

(event `/Game/Tyler/SteamPunk_BuildingMechanic/Interfaces/BPI_Interactable.ShowAttachmentPoints`
  (for _array_element (`|MakeArray` (`self.Front`) (`self.Top`) (`self.Bottom`) (`self.Back`))
    (`SceneComponent.SetVisibility` (`SceneComponent.GetChildComponent` _array_element 0) true false)))

(event `/Game/Tyler/SteamPunk_BuildingMechanic/Interfaces/BPI_Interactable.DropObject`
  (set `/Game/FirstPerson/Blueprints/BP_FirstPersonCharacter.IsObjectInHand?` false (`self.BP_FirstPersonRef`))
  (`SceneComponent.K2_DetachFromComponent` (`self.BaseMesh`) "KeepWorld" "KeepWorld" "KeepWorld" true)
  (`PrimitiveComponent.SetSimulatePhysics` (`self.BaseMesh`) true))

(fn `AddChildRefrence`
  (params (`Child Object` :type "/Game/Tyler/SteamPunk_BuildingMechanic/Blueprints/BP_Base_Object Object Reference"))
  (`KismetArrayLibrary.Array_AddUnique` (`self.AttachedChildernArray`) `Child Object`))

(fn `CanBeDetached?`
  (returns (`CanBeDetached?` :type Boolean))
  (return (== (`KismetArrayLibrary.Array_Length` (`self.AttachedChildernArray`)) 0)))

(fn `RemoveChildRefrence`
  (params (`Child Object` :type "/Game/Tyler/SteamPunk_BuildingMechanic/Blueprints/BP_Base_Object Object Reference"))
  (`/Engine/EditorBlueprintResources/StandardMacros.IsValid` (`self.ParentObject`)
    (:`Is Valid`
      (`KismetArrayLibrary.Array_RemoveItem` (`/Game/Tyler/SteamPunk_BuildingMechanic/Blueprints/BP_Base_Object.AttachedChildernArray` (`self.ParentObject`)) self))))

(fn `UserConstructionScript`
  (for _array_element (`|MakeArray` (`self.Front`) (`self.Top`) (`self.Bottom`) (`self.Back`))
    (`SceneComponent.SetVisibility` (`SceneComponent.GetChildComponent` _array_element 0) false false)))